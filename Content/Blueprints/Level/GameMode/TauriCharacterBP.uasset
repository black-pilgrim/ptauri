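; Multiplayer third-person shooter character with a socket-attached weapon, health, firing, reloading and ironsights.
; Inputs call Server events that relay to Multicast events, toggling ThirdPerson_AnimBP flags and ironsight walk speed.
; On authority, firing line-traces from the follow camera, damages hit TauriCharacterBPs and multicasts the impact for bullet-hole decals.
; P and O keys adjust health directly; CreateHUD and the construction script are empty.
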(event EventBeginPlay
  ;[1 1 1] GameSetup
  (CallFunction|SetWalkingSpeeds)
  (CallFunction|SetAnimInstance)
  (CallFunction|EquipWeapon))

(event Custom|ServerUpdateHealth
  (params (Damage :type Integer))
  ;[1 1 1] Update Health
  (Networking|SwitchHasAuthority
    (:Authority
      (Variables|Default|SetCurrentHealth (- (Variables|Default|GetCurrentHealth) Damage)))))

(event Custom|ServerStopFiring
  ;[1 1 1] Fire Weapon
  (Networking|SwitchHasAuthority
    (:Authority
      (CallFunction|MultiCastStopFiring))))

(event Custom|MultiCastStopFiring
  ;[1 1 1] Fire Weapon
  (CallFunction|AnimateFiring))

(event Custom|ServerReload
  ;[1 1 1] Reload Weapon
  (CallFunction|MulticastReload))

(event Custom|MulticastReload
  ;[1 1 1] Reload Weapon
  (bind _asthird_person_anim_bp (Utilities|Casting|CastToThirdPerson_AnimBP (Variables|Default|GetAnimationInstance)))
  (Variables|/Game/Objects/Character/Animations/ThirdPerson_AnimBP.ThirdPerson_AnimBP_C|SetReloading? _asthird_person_anim_bp true))

(event Custom|ServerIronsight
  ;[1 1 1] Activate Ironsight
  (CallFunction|MulticastIronsight))

(event Custom|MulticastIronsight
  (bind _charactermovement (Variables|Character|GetCharacterMovement))
  ;[1 1 1] Activate Ironsight
  (bind _asthird_person_anim_bp (Utilities|Casting|CastToThirdPerson_AnimBP (Variables|Default|GetAnimationInstance)))
  (if (Variables|/Game/Objects/Character/Animations/ThirdPerson_AnimBP.ThirdPerson_AnimBP_C|GetWeaponEquipped? _asthird_person_anim_bp) ; Only Slow down, when Weapon equipped
    (bind _output_get (Variables|/Game/Objects/Character/Animations/ThirdPerson_AnimBP.ThirdPerson_AnimBP_C|SetIronsightActive? _asthird_person_anim_bp (not (Variables|/Game/Objects/Character/Animations/ThirdPerson_AnimBP.ThirdPerson_AnimBP_C|GetIronsightActive? _asthird_person_anim_bp))))
    (if _output_get
      (Variables|/Script/Engine.CharacterMovementComponent|SetMaxWalkSpeed _charactermovement (Variables|Default|GetIronsightSpeed))
      (else
        (Variables|/Script/Engine.CharacterMovementComponent|SetMaxWalkSpeed _charactermovement (Variables|Default|GetWalkWeaponSpeed))))))

(event Custom|ServerFire
  ;[1 1 1] Fire Weapon
  (Networking|SwitchHasAuthority
    (:Authority
      (bind (_impactpoint _returnvalue) (CallFunction|ShootandDamage))
      (CallFunction|MulticastFire _impactpoint _returnvalue))))

(event Custom|MulticastFire
  (params (ImpactPoint :type Vector) (ImpactNormalRotator :type Rotator))
  ;[1 1 1] Fire Weapon
  (CallFunction|AnimateFiring)
  (CallFunction|SpawnBulletHoleDecal ImpactPoint ImpactNormalRotator))

(event Input|KeyboardEvents|R
  (params (Key :type Key%20Structure :default "AnyKey"))
  ;[1 1 1] Keyboard
  (:Pressed
    (CallFunction|ServerReload)))

(event Input|KeyboardEvents|P
  (params (Key :type Key%20Structure :default "AnyKey"))
  ;[1 1 1] Keyboard
  (:Pressed
    (CallFunction|ServerUpdateHealth 5)))

(event Input|MouseEvents|RightMouseButton
  (params (Key :type Key%20Structure :default "AnyKey"))
  ;[1 1 1] Mouse
  (:Pressed
    (CallFunction|ServerIronsight :!label _label))
  (:Released
    (goto _label)))

(event Input|KeyboardEvents|O
  (params (Key :type Key%20Structure :default "AnyKey"))
  ;[1 1 1] Keyboard
  (:Pressed
    (CallFunction|ServerUpdateHealth -5)))

(event Input|MouseEvents|LeftMouseButton
  (params (Key :type Key%20Structure :default "AnyKey"))
  ;[1 1 1] Mouse
  (:Pressed
    (CallFunction|ServerFire))
  (:Released
    (CallFunction|ServerStopFiring)))

(fn ConstructionScript)

(fn SetWalkingSpeeds
  (Variables|/Script/Engine.CharacterMovementComponent|SetMaxWalkSpeed (Variables|Character|GetCharacterMovement) (Variables|Default|GetWalkSpeed))
  (Variables|Default|SetWalkWeaponSpeed (* (Variables|Default|GetWalkSpeed) 0.75))
  (Variables|Default|SetIronsightSpeed (* (Variables|Default|GetWalkWeaponSpeed) 0.75))
  (return))

(fn CreateHUD)

(fn SetAnimInstance
  (Variables|Default|SetAnimationInstance (Components|SkeletalMesh|GetAnimInstance (Variables|Character|GetMesh)))
  (return))

(fn EquipWeapon
  (bind _returnvalue (AddComponent|AddStaticMeshComponent false))
  (bind _output_get (Variables|Default|SetCurrentWeapon _returnvalue))
  (Class|SceneComponent|Attachto _output_get (Variables|Character|GetMesh) "Weapon_R_Socket" "KeepRelativeOffset" true))

(fn AnimateFiring
  (bind _asthird_person_anim_bp (Utilities|Casting|CastToThirdPerson_AnimBP (Variables|Default|GetAnimationInstance))
    (:then
      (Variables|/Game/Objects/Character/Animations/ThirdPerson_AnimBP.ThirdPerson_AnimBP_C|SetShooting? _asthird_person_anim_bp (not (Variables|/Game/Objects/Character/Animations/ThirdPerson_AnimBP.ThirdPerson_AnimBP_C|GetShooting? _asthird_person_anim_bp))))
    (:CastFailed
      _))
  (return))

(fn SpawnBulletHoleDecal
  (params (Location :type Vector) (Rotation :type Rotator))
  (bind _returnvalue (Game|SpawnActorfromClass "/Script/Engine.DecalActor" (Math|Transform|MakeTransform Location Rotation "20.000000,20.000000,20.000000") "Undefined" 0 0))
  (Rendering|Components|Decal|SetDecalMaterial (Variables|/Script/Engine.DecalActor|GetDecal _returnvalue) "/Game/Blueprints/Level/Weapons/bullethole_Mat.bullethole_Mat")
  (return))

(fn ShootandDamage
  (bind _followcamera (Variables|Default|GetFollowCamera))
  (bind _returnvalue (Transformation|GetWorldLocation _followcamera))
  (bind _outhit (Collision|LineTraceByChannel _returnvalue (+ _returnvalue (* (Math|Vector|GetForwardVector _followcamera) 50000)) "TraceTypeQuery2" false 0 "ForDuration"))
  (LocalVariables|SetImpactPt (.ImpactPoint (Collision|BreakHitResult _outhit)))
  (LocalVariables|SetImpactNormal (.ImpactNormal (Collision|BreakHitResult _outhit)))
  (bind _astauri_character_bp (Utilities|Casting|CastToTauriCharacterBP (.HitActor (Collision|BreakHitResult _outhit)))
    (:then
      (LocalVariables|SetTarget _astauri_character_bp)
      (Variables|TauriCharacterBP_C|SetCurrentHealth (LocalVariables|GetTarget) (- (Variables|TauriCharacterBP_C|GetCurrentHealth (LocalVariables|GetTarget)) 10)))
    (:CastFailed
      _))
  (return (LocalVariables|GetImpactPt) (Math|Conversions|RotationFromXVector (LocalVariables|GetImpactNormal))))

(fn HealthStates
  (return (Variables|Default|GetCurrentHealth)))